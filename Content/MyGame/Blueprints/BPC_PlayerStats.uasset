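; Stats component for the player, dummy and AI characters, tracking health, stamina, XP and level.
; BeginPlay waits a tick, casts the owner to set CharacterType, then initializes the player HUD or the owner's health bar widget.
; Stat functions push changes straight to widgets; only DecreaseHealth supports all three owner types, returning true at zero health.
; XP overflow is discarded on level-up, which raises MaxXP and plays sounds.
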(event EventBeginPlay
  (Utilities|FlowControl|DelayUntilNextTick)
  (bind _asbp_third_person_character (Utilities|Casting|CastToBP_ThirdPersonCharacter (Components|GetOwner))
    (:then
      (Variables|Default|SetPlayer%20Character%20BP _asbp_third_person_character)
      (Variables|Default|SetisPlayer true)
      (Variables|Default|SetCharacter%20Type "NewEnumerator0")
      (Progress|SetPercent (Variables|/Game/MyGame/UI/WB_HUD.WB_HUD_C|GetStaminaBar (Variables|/Game/ThirdPerson/Blueprints/BP_ThirdPersonCharacter.BP_ThirdPersonCharacter_C|GetHUD%20Widget (Variables|Default|GetPlayer%20Character%20BP))) (/ (Variables|Stamina|GetCurrent%20Stamina) (Variables|Stamina|GetMax%20Stamina))))
    (:CastFailed
      (bind _asbp_dummy (Utilities|Casting|CastToBP_Dummy (Components|GetOwner))
        (:then
          (Variables|Default|SetDummy%20BP _asbp_dummy)
          (Variables|Default|SetisPlayer false)
          (Variables|Default|SetCharacter%20Type "NewEnumerator1"))
        (:CastFailed
          (bind _asbp_ai (Utilities|Casting|CastToBP_AI (Components|GetOwner)))
          (Variables|Default|SetAI%20BP _asbp_ai)
          (Variables|Default|SetCharacter%20Type "NewEnumerator2")))))
  (Progress|SetPercent (Utilities|Select :Index (Variables|Default|GetCharacter%20Type) :NewEnumerator0 (Variables|/Game/MyGame/UI/WB_HUD.WB_HUD_C|GetHealthBar (Variables|/Game/ThirdPerson/Blueprints/BP_ThirdPersonCharacter.BP_ThirdPersonCharacter_C|GetHUD%20Widget (Variables|Default|GetPlayer%20Character%20BP))) :NewEnumerator1 (Variables|/Game/MyGame/UI/WB_DummyHealth.WB_DummyHealth_C|GetHealthBar (Variables|/Game/MyGame/Blueprints/BP_Dummy.BP_Dummy_C|GetHealth%20Bar%20UI (Variables|Default|GetDummy%20BP))) :NewEnumerator2 (Variables|/Game/MyGame/UI/WB_DummyHealth.WB_DummyHealth_C|GetHealthBar (Variables|/Game/MyGame/AI/BP_AI.BP_AI_C|GetHealth%20Bar%20UI (Variables|Default|GetAI%20BP)))) (/ (Variables|Health|GetCurrent%20Health) (Variables|Health|GetMax%20Health)))
  (Rendering|Components|TextRender|SetText (Utilities|Select :Index (Variables|Default|GetCharacter%20Type) :NewEnumerator0 (Variables|/Game/MyGame/UI/WB_HUD.WB_HUD_C|GetHealthText (Variables|/Game/ThirdPerson/Blueprints/BP_ThirdPersonCharacter.BP_ThirdPersonCharacter_C|GetHUD%20Widget (Variables|Default|GetPlayer%20Character%20BP))) :NewEnumerator1 (Variables|/Game/MyGame/UI/WB_DummyHealth.WB_DummyHealth_C|GetHealthText (Variables|/Game/MyGame/Blueprints/BP_Dummy.BP_Dummy_C|GetHealth%20Bar%20UI (Variables|Default|GetDummy%20BP))) :NewEnumerator2 (Variables|/Game/MyGame/UI/WB_DummyHealth.WB_DummyHealth_C|GetHealthText (Variables|/Game/MyGame/AI/BP_AI.BP_AI_C|GetHealth%20Bar%20UI (Variables|Default|GetAI%20BP)))) (Utilities|Text|ToText(Float) (Variables|Health|GetCurrent%20Health) "HalfToEven"))
  (if (Variables|Default|GetisPlayer)
    (Progress|SetPercent (Variables|/Game/MyGame/UI/WB_HUD.WB_HUD_C|GetXPBar (Variables|/Game/ThirdPerson/Blueprints/BP_ThirdPersonCharacter.BP_ThirdPersonCharacter_C|GetHUD%20Widget (Variables|Default|GetPlayer%20Character%20BP))) (/ (Variables|XP|GetXP) (Variables|XP|GetMax%20XP)))
    (Rendering|Components|TextRender|SetText (Variables|/Game/MyGame/UI/WB_HUD.WB_HUD_C|GetXPText (Variables|/Game/ThirdPerson/Blueprints/BP_ThirdPersonCharacter.BP_ThirdPersonCharacter_C|GetHUD%20Widget (Variables|Default|GetPlayer%20Character%20BP))) (Utilities|Text|FormatText "{Current XP} / {Max XP}" (Variables|XP|GetXP) (Variables|XP|GetMax%20XP)))
    (Rendering|Components|TextRender|SetText (Variables|/Game/MyGame/UI/WB_HUD.WB_HUD_C|GetLevelText (Variables|/Game/ThirdPerson/Blueprints/BP_ThirdPersonCharacter.BP_ThirdPersonCharacter_C|GetHUD%20Widget (Variables|Default|GetPlayer%20Character%20BP))) (Utilities|Text|ToText(Integer) (Variables|XP|GetLevel)))))

(fn DecreaseHealth
  (params (Dammage :type Float%20%28double-precision%29))
  (if (not (<= (Variables|Health|GetCurrent%20Health) 0.0))
    (bind _output_get (Variables|Health|SetCurrent%20Health (- (Variables|Health|GetCurrent%20Health) Dammage)))
    (Progress|SetPercent (Utilities|Select :Index (Variables|Default|GetCharacter%20Type) :NewEnumerator0 (Variables|/Game/MyGame/UI/WB_HUD.WB_HUD_C|GetHealthBar (Variables|/Game/ThirdPerson/Blueprints/BP_ThirdPersonCharacter.BP_ThirdPersonCharacter_C|GetHUD%20Widget (Variables|Default|GetPlayer%20Character%20BP))) :NewEnumerator1 (Variables|/Game/MyGame/UI/WB_DummyHealth.WB_DummyHealth_C|GetHealthBar (Variables|/Game/MyGame/Blueprints/BP_Dummy.BP_Dummy_C|GetHealth%20Bar%20UI (Variables|Default|GetDummy%20BP))) :NewEnumerator2 (Variables|/Game/MyGame/UI/WB_DummyHealth.WB_DummyHealth_C|GetHealthBar (Variables|/Game/MyGame/AI/BP_AI.BP_AI_C|GetHealth%20Bar%20UI (Variables|Default|GetAI%20BP)))) (/ _output_get (Variables|Health|GetMax%20Health)))
    (Rendering|Components|TextRender|SetText (Utilities|Select :Index (Variables|Default|GetCharacter%20Type) :NewEnumerator0 (Variables|/Game/MyGame/UI/WB_HUD.WB_HUD_C|GetHealthText (Variables|/Game/ThirdPerson/Blueprints/BP_ThirdPersonCharacter.BP_ThirdPersonCharacter_C|GetHUD%20Widget (Variables|Default|GetPlayer%20Character%20BP))) :NewEnumerator1 (Variables|/Game/MyGame/UI/WB_DummyHealth.WB_DummyHealth_C|GetHealthText (Variables|/Game/MyGame/Blueprints/BP_Dummy.BP_Dummy_C|GetHealth%20Bar%20UI (Variables|Default|GetDummy%20BP))) :NewEnumerator2 (Variables|/Game/MyGame/UI/WB_DummyHealth.WB_DummyHealth_C|GetHealthText (Variables|/Game/MyGame/AI/BP_AI.BP_AI_C|GetHealth%20Bar%20UI (Variables|Default|GetAI%20BP)))) (Utilities|Text|ToText(Float) (Variables|Health|GetCurrent%20Health) "HalfToEven"))
    (if (<= (Variables|Health|GetCurrent%20Health) 0.0)
      _
      (else
        (return false))))
  (return true))

(fn IncreasseMaxHealth
  (params (Health%20Incremention :type Float%20%28double-precision%29))
  (bind _player_character_bp (Variables|Default|GetPlayer%20Character%20BP))
  (bind _hud_widget (Variables|/Game/ThirdPerson/Blueprints/BP_ThirdPersonCharacter.BP_ThirdPersonCharacter_C|GetHUD%20Widget _player_character_bp))
  (Variables|Health|SetMax%20Health (+ (Variables|Health|GetMax%20Health) Health%20Incremention))
  (Progress|SetPercent (Variables|/Game/MyGame/UI/WB_HUD.WB_HUD_C|GetHealthBar _hud_widget) (/ (Variables|Health|GetCurrent%20Health) (Variables|Health|GetMax%20Health)))
  (Rendering|Components|TextRender|SetText (Variables|/Game/MyGame/UI/WB_HUD.WB_HUD_C|GetHealthText _hud_widget) (Utilities|Text|ToText(Float) (Variables|Health|GetCurrent%20Health) "HalfToEven")))

(fn DecreaseStamina
  (params (Stamina%20Depleted :type Float%20%28double-precision%29))
  (if (not (<= (Variables|Stamina|GetCurrent%20Stamina) 0.0))
    (Variables|Stamina|SetCurrent%20Stamina (- (Variables|Stamina|GetCurrent%20Stamina) Stamina%20Depleted))
    (Progress|SetPercent (Variables|/Game/MyGame/UI/WB_HUD.WB_HUD_C|GetStaminaBar (Variables|/Game/ThirdPerson/Blueprints/BP_ThirdPersonCharacter.BP_ThirdPersonCharacter_C|GetHUD%20Widget (Variables|Default|GetPlayer%20Character%20BP))) (/ (Variables|Stamina|GetCurrent%20Stamina) (Variables|Stamina|GetMax%20Stamina)))
    (if (<= (Variables|Health|GetCurrent%20Health) 0.0)
      _
      (else
        (return false))))
  (return true))

(fn IncreaseMaxStamina
  (params (Added%20Stamina :type Float%20%28double-precision%29))
  (Variables|Stamina|SetMax%20Stamina (+ (Variables|Stamina|GetMax%20Stamina) Added%20Stamina))
  (Progress|SetPercent (Variables|/Game/MyGame/UI/WB_HUD.WB_HUD_C|GetStaminaBar (Variables|/Game/ThirdPerson/Blueprints/BP_ThirdPersonCharacter.BP_ThirdPersonCharacter_C|GetHUD%20Widget (Variables|Default|GetPlayer%20Character%20BP))) (/ (Variables|Stamina|GetCurrent%20Stamina) (Variables|Stamina|GetMax%20Stamina))))

(fn IncreaseHealth
  (params (Added%20Health :type Float%20%28double-precision%29))
  (bind _player_character_bp (Variables|Default|GetPlayer%20Character%20BP))
  (bind _hud_widget (Variables|/Game/ThirdPerson/Blueprints/BP_ThirdPersonCharacter.BP_ThirdPersonCharacter_C|GetHUD%20Widget _player_character_bp))
  (Variables|Health|SetCurrent%20Health (+ (Variables|Health|GetCurrent%20Health) Added%20Health))
  (if (> (Variables|Health|GetCurrent%20Health) (Variables|Health|GetMax%20Health))
    (Variables|Health|SetCurrent%20Health (Variables|Health|GetMax%20Health)))
  (Progress|SetPercent (Variables|/Game/MyGame/UI/WB_HUD.WB_HUD_C|GetHealthBar _hud_widget) (/ (Variables|Health|GetCurrent%20Health) (Variables|Health|GetMax%20Health)))
  (Rendering|Components|TextRender|SetText (Variables|/Game/MyGame/UI/WB_HUD.WB_HUD_C|GetHealthText _hud_widget) (Utilities|Text|ToText(Float) (Variables|Health|GetCurrent%20Health) "HalfToEven")))

(fn IncreaseStamina
  (params (Added%20Stamina :type Float%20%28double-precision%29))
  (Variables|Stamina|SetCurrent%20Stamina (+ (Variables|Stamina|GetCurrent%20Stamina) Added%20Stamina))
  (if (> (Variables|Stamina|GetCurrent%20Stamina) (Variables|Stamina|GetMax%20Stamina))
    (Variables|Stamina|SetCurrent%20Stamina (Variables|Stamina|GetMax%20Stamina)))
  (Progress|SetPercent (Variables|/Game/MyGame/UI/WB_HUD.WB_HUD_C|GetStaminaBar (Variables|/Game/ThirdPerson/Blueprints/BP_ThirdPersonCharacter.BP_ThirdPersonCharacter_C|GetHUD%20Widget (Variables|Default|GetPlayer%20Character%20BP))) (/ (Variables|Stamina|GetCurrent%20Stamina) (Variables|Stamina|GetMax%20Stamina))))

(fn IncreaseXP
  (params (Added%20XP :type Float%20%28double-precision%29))
  (Variables|XP|SetXP (+ (Variables|XP|GetXP) Added%20XP))
  (if (>= (Variables|XP|GetXP) (Variables|XP|GetMax%20XP))
    (LevelAndXP|IncreaseLevel 1))
  (Progress|SetPercent (Variables|/Game/MyGame/UI/WB_HUD.WB_HUD_C|GetXPBar (Variables|/Game/ThirdPerson/Blueprints/BP_ThirdPersonCharacter.BP_ThirdPersonCharacter_C|GetHUD%20Widget (Variables|Default|GetPlayer%20Character%20BP))) (/ (Variables|XP|GetXP) (Variables|XP|GetMax%20XP)))
  (Rendering|Components|TextRender|SetText (Variables|/Game/MyGame/UI/WB_HUD.WB_HUD_C|GetXPText (Variables|/Game/ThirdPerson/Blueprints/BP_ThirdPersonCharacter.BP_ThirdPersonCharacter_C|GetHUD%20Widget (Variables|Default|GetPlayer%20Character%20BP))) (Utilities|Text|FormatText "{Current XP} / {Max XP}" (Variables|XP|GetXP) (Variables|XP|GetMax%20XP))))

(fn IncreaseLevel
  (params (Added%20Level :type Integer))
  (Variables|XP|SetLevel (+ (Variables|XP|GetLevel) Added%20Level))
  (Variables|XP|SetMax%20XP (+ (Variables|XP|GetMax%20XP) 1.5e+02))
  (Variables|XP|SetXP 0.0)
  (Rendering|Components|TextRender|SetText (Variables|/Game/MyGame/UI/WB_HUD.WB_HUD_C|GetLevelText (Variables|/Game/ThirdPerson/Blueprints/BP_ThirdPersonCharacter.BP_ThirdPersonCharacter_C|GetHUD%20Widget (Variables|Default|GetPlayer%20Character%20BP))) (Utilities|Text|ToText(Integer) (Variables|XP|GetLevel)))
  (Audio|PlaySound2D "/Game/MyGame/Audio/LevelUp/level-up-1.level-up-1" 1.0 1.0 0.0 0 0)
  (Audio|PlaySound2D "/Game/MyGame/Audio/LevelUp/level-up-2.level-up-2" 1.0 1.0 0.0 0 0))