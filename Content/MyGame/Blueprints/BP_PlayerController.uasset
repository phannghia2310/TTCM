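; Player controller that toggles the pause menu when the IA_PauseGame input action starts.
; Opening creates WB_PauseMenu, adds it to the viewport, switches to UI-only input focused on the widget, shows the cursor and pauses the game.
; The same action's closing branch removes and clears the widget, restores game-only input, hides the cursor and unpauses, with IsPauseMenuOpen tracking the state.
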(event Input|EnhancedActionEvents|EnhancedInputActionIA_PauseGame
  (params (ActionValue :type Boolean) (ElapsedSeconds :type Float%20%28double-precision%29) (TriggeredSeconds :type Float%20%28double-precision%29) (InputAction :type Input%20Action%20Object%20Reference :default "/Game/MyGame/Characters/Input/Actions/IA_PauseGame.IA_PauseGame"))
  ;[0.05098 0.05098 0.05098] Pause Game
  (:Started
    (if (Variables|Default|GetIsPauseMenuOpen)
      (Variables|Default|SetIsPauseMenuOpen false)
      (Widget|RemovefromParent (Variables|Default|GetWB_PauseMenu))
      (Variables|Default|SetWB_PauseMenu 0)
      (Input|SetInputModeGameOnly self)
      (Variables|Default|SetbShowMouseCursor false)
      (Game|SetGamePaused false)
      (else
        (Variables|Default|SetIsPauseMenuOpen true)
        (bind _returnvalue (UserInterface|CreateWidget "/Game/MyGame/UI/WB_PauseMenu.WB_PauseMenu_C" (Game|GetPlayerController 0)))
        (bind _output_get (Variables|Default|SetWB_PauseMenu _returnvalue))
        (UserInterface|Viewport|AddtoViewport _output_get 0)
        (Input|SetInputModeUIOnly self (Variables|Default|GetWB_PauseMenu) "DoNotLock")
        (Variables|Default|SetbShowMouseCursor true)
        (Game|SetGamePaused true)))))

(event EventBeginPlay)

(event EventTick
  (params (DeltaSeconds :type Float%20%28single-precision%29)))

(fn ConstructionScript)